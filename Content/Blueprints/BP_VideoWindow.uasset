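; BP_VideoWindow is an actor that rises to a target height and then plays a video.
; StartMove calls Move, which nudges the actor up one unit locally and re-arms itself on a short looping timer.
; A GoalVerification macro compares world Z to HeightToBeClimbed; once reached, PlayMovie opens the Video source on the MediaPlayer.
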(fn `Move`
  (`self.K2_AddActorLocalTransform` self (`KismetMathLibrary.MakeTransform` (0.0 0.0 1.0)) false false)
  (`self.GoalVerification`
    (:`true`
      (`self.PlayMovie`))
    (:`false`
      (`KismetSystemLibrary.K2_SetTimer` self "Move" 0.01))))

(fn `PlayMovie`
  (`MediaPlayer.OpenSource` (`self.MediaPlayer`) (`self.Video`)))

(fn `StartMove`
  (`self.Move`))

(fn `UserConstructionScript`)