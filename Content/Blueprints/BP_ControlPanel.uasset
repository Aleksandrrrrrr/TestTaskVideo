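; BP_ControlPanel is an interactable panel whose progress builds with repeated interactions to open the level's video windows.
; Each Interact adds a click value through ChangeProgress, while Tick drains progress at SpeedMoveWindow whenever it sits between zero and one.
; At full progress, ChangeProgress calls StartMove on every BP_VideoWindow and pushes the value to its progress bar widget, which is updated only in that branch.
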(event `self.ReceiveBeginPlay`
  (`self.ChangeProgress` (`self.ValueForSuccess`)))

(event `self.ReceiveTick`
  (params (DeltaSeconds :type "Float (single-precision)"))
  (bind _valueforsuccess (`self.ValueForSuccess`))
  (if (and (> _valueforsuccess 0.0) (< _valueforsuccess 1.0))
    (`self.ChangeProgress` (* DeltaSeconds (`self.SpeedMoveWindow`) -1.0))))

(fn `ChangeProgress`
  (params (Value :type "Float (double-precision)"))
  (set `self.ValueForSuccess` (+ (`self.ValueForSuccess`) (`local.Value`)))
  (if (>= (`self.ValueForSuccess`) 1.0)
    (`self.OpenVideoWindow`)
    (bind _aswidget_progress_bar (cast `/Game/Widgets/Widget_ProgressBar` (`WidgetComponent.GetUserWidgetObject` (`self.ProgressBar`))))
    (`/Game/Widgets/Widget_ProgressBar.ChangeProgressValue` _aswidget_progress_bar (`self.ValueForSuccess`))))

(fn `Interact`
  (returns (Result :type Boolean))
  (`self.ChangeProgress` (`self.ValueOfSuccessfulClick`))
  (return true))

(fn `OpenVideoWindow`
  (bind _outactors (`GameplayStatics.GetAllActorsOfClass` "/Game/Blueprints/BP_VideoWindow.BP_VideoWindow_C"))
  (for _array_element _outactors
    (`/Game/Blueprints/BP_VideoWindow.StartMove` _array_element)))

(fn `UserConstructionScript`)